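; Test-level trigger zone manager that builds an apartment from swappable room actors and tracks which room is entered.
; BeginPlay spawns the first bathroom, kitchen, living room and office variant, then binds enter and leave dispatchers for those rooms and the floor.
; Enter events update room state and push it to the HUD_TriggerZones UI; both enter and leave print debug messages.
; Update functions swap a room by destroying the previous variant's actors and spawning the requested one.
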(event `self.ReceiveBeginPlay`
  ;[1 1 1] Area 2
  ;;[1 1 1] Spawn Rooms
  (`|SpawnActorFromClass` (`|GetArrayItem` (`self.Bathrooms`)) (`self.BathroomTransform`) "Undefined" "MultiplyWithRoot" null null)
  (`|SpawnActorFromClass` (`|GetArrayItem` (`self.Kitchens`)) (`self.KitchenTransform`) "Undefined" "MultiplyWithRoot" null null)
  (`|SpawnActorFromClass` (`|GetArrayItem` (`self.LivingRooms`)) (`self.LivingRoomTransform`) "Undefined" "MultiplyWithRoot" null null)
  (`|SpawnActorFromClass` (`|GetArrayItem` (`self.Offices`)) (`self.OfficeTransform`) "Undefined" "MultiplyWithRoot" null null)
  ;;[1 1 1] Enter a room
  (add `self.ED_EnterFloor ` (delegate `EnterFloor`))
  (add `self.ED_EnterBathroom` (delegate `EnterBathroom`))
  (add `self.ED_EnterKitchen` (delegate `EnterKitchen`))
  (add `self.ED_EnterLivingRoom` (delegate `EnterLivingRoom`))
  (add `self.ED_EnterOffice` (delegate `EnterOffice`))
  ;;[1 1 1] Leave a room
  (add `self.ED_LeaveFloor` (delegate `LeaveFloor`))
  (add `self.ED_LeaveBathroom` (delegate `LeaveBathroom`))
  (add `self.ED_LeaveKitchen` (delegate `LeaveKitchen`))
  (add `self.ED_LeaveLivingRoom` (delegate `LeaveLivingRoom`))
  (add `self.ED_LeaveOffice` (delegate `LeaveOffice`)))

(event `EnterFloor`
  ;[1 1 1] Area 2
  ;;[1 1 1] Enter a room
  (set `self.InARoom` false)
  (set `self.CurrentRoom` "Floor")
  (`self.EnterRoom` :!label _label)
  (`self.UpdateUI`))

(event `EnterBathroom`
  ;[1 1 1] Area 2
  ;;[1 1 1] Enter a room
  (set `self.InARoom` true)
  (set `self.CurrentRoom` "Bathroom")
  (goto _label))

(event `EnterKitchen`
  ;[1 1 1] Area 2
  ;;[1 1 1] Enter a room
  (set `self.InARoom` true)
  (set `self.CurrentRoom` "Kitchen")
  (goto _label))

(event `EnterLivingRoom`
  ;[1 1 1] Area 2
  ;;[1 1 1] Enter a room
  (set `self.InARoom` true)
  (set `self.CurrentRoom` "Living room")
  (goto _label))

(event `EnterOffice`
  ;[1 1 1] Area 2
  ;;[1 1 1] Enter a room
  (set `self.InARoom` true)
  (set `self.CurrentRoom` "Office")
  (goto _label))

(event `LeaveFloor`
  ;[1 1 1] Area 2
  ;;[1 1 1] Leave a room
  (set `self.LastRoom` "Floor")
  (`self.LeaveRoom` :!label _label_2))

(event `LeaveBathroom`
  ;[1 1 1] Area 2
  ;;[1 1 1] Leave a room
  (set `self.LastRoom` "Bathroom")
  (goto _label_2))

(event `LeaveKitchen`
  ;[1 1 1] Area 2
  ;;[1 1 1] Leave a room
  (set `self.LastRoom` "Kitchen")
  (goto _label_2))

(event `LeaveLivingRoom`
  ;[1 1 1] Area 2
  ;;[1 1 1] Leave a room
  (set `self.LastRoom` "Living room")
  (goto _label_2))

(event `LeaveOffice`
  ;[1 1 1] Area 2
  ;;[1 1 1] Leave a room
  (set `self.LastRoom` "Office")
  (goto _label_2))

(fn `EnterRoom`
  (`KismetSystemLibrary.PrintString` (`KismetStringLibrary.Concat_StrStr` "Enter " (`self.CurrentRoom`)) true true (struct :`G` 0.244792 :`B` 0.059479 :`A` 1.0) 5.0))

(fn `LeaveRoom`
  (`KismetSystemLibrary.PrintString` (`KismetStringLibrary.Concat_StrStr` "Leave " (`self.LastRoom`)) true true (struct :`R` 0.244792 :`G` 0.0339 :`B` 0.014395 :`A` 1.0) 5.0))

(fn `Update Bathroom`
  (params (NewRoom :type Integer))
  (bind _bathrooms (`self.Bathrooms`))
  (bind _outactors (`GameplayStatics.GetAllActorsOfClass` (`|GetArrayItem` _bathrooms (- NewRoom 1))))
  (`self.K2_DestroyActor` _outactors)
  (`|SpawnActorFromClass` (`|GetArrayItem` _bathrooms NewRoom) (`self.BathroomTransform`) "Undefined" "MultiplyWithRoot" null null))

(fn `Update Kitchen`
  (params (NewRoom :type Integer))
  (bind _kitchens (`self.Kitchens`))
  (bind _outactors (`GameplayStatics.GetAllActorsOfClass` (`|GetArrayItem` _kitchens (- NewRoom 1))))
  (`self.K2_DestroyActor` _outactors)
  (`|SpawnActorFromClass` (`|GetArrayItem` _kitchens NewRoom) (`self.KitchenTransform`) "Undefined" "MultiplyWithRoot" null null))

(fn `Update LivingRoom`
  (params (NewRoom :type Integer))
  (bind _livingrooms (`self.LivingRooms`))
  (bind _outactors (`GameplayStatics.GetAllActorsOfClass` (`|GetArrayItem` _livingrooms (- NewRoom 1))))
  (`self.K2_DestroyActor` _outactors)
  (`|SpawnActorFromClass` (`|GetArrayItem` _livingrooms NewRoom) (`self.LivingRoomTransform`) "Undefined" "MultiplyWithRoot" null null))

(fn `Update Office`
  (params (NewRoom :type Integer))
  (bind _offices (`self.Offices`))
  (bind _outactors (`GameplayStatics.GetAllActorsOfClass` (`|GetArrayItem` _offices (- NewRoom 1))))
  (`self.K2_DestroyActor` _outactors)
  (`|SpawnActorFromClass` (`|GetArrayItem` _offices NewRoom) (`self.OfficeTransform`) "Undefined" "MultiplyWithRoot" null null))

(fn `UpdateUI`
  (bind _ashud_trigger_zones (cast `/Game/Levels/Testlevel_TriggerZones_Jordan/HUD_TriggerZones` (`PlayerController.GetHUD` (`GameplayStatics.GetPlayerController` 0))))
  (bind _ui_ref (`/Game/Levels/Testlevel_TriggerZones_Jordan/HUD_TriggerZones.UI_Ref` _ashud_trigger_zones))
  (`/Game/Levels/Testlevel_TriggerZones_Jordan/WP_UI.SetCurrentApartmentRoom` _ui_ref (`self.CurrentRoom`))
  (`/Game/Levels/Testlevel_TriggerZones_Jordan/WP_UI.SetRoomState` _ui_ref (`self.InARoom`))
  (`/Game/Levels/Testlevel_TriggerZones_Jordan/WP_UI.UpdateCurrentApartmentRoomUI` _ui_ref))

(fn `UserConstructionScript`)
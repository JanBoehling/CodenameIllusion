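; BP_DebugRoomTrigger is a debug trigger box that updates one room (bathroom, kitchen, living room or office) when the player walks into it.
; On BeginPlay it caches the first BP_TriggerZones actor found in the level.
; When the player pawn overlaps the box, RoomToUpdate selects which update function to call on that actor.
; Per-room booleans limit each trigger instance to a single update, confirmed by a printed message.
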(event `self.ReceiveBeginPlay`
  ;[1 1 1] BP_TriggerZones Ref erhalten
  (bind _outactors (`GameplayStatics.GetAllActorsOfClass` "/Game/Levels/Testlevel_TriggerZones_Jordan/BP_TriggerZones.BP_TriggerZones_C"))
  (set `self.TriggerZonesRef` (`|GetArrayItem` _outactors)))

(event `self.Box.OnComponentBeginOverlap`
  (params (OverlappedComponent :type "PrimitiveComponent Object Reference") (OtherActor :type "Actor Object Reference") (OtherComp :type "PrimitiveComponent Object Reference") (OtherBodyIndex :type Integer) (bFromSweep :type Boolean) (SweepResult :type "HitResult Structure (by ref)"))
  (bind _triggerzonesref (`self.TriggerZonesRef`))
  (bind _roomtoupdate (`self.RoomToUpdate`))
  ;[1 1 1] Updae Room
  ;;[1 1 1] Is it the player?
  (if (== OtherActor (`GameplayStatics.GetPlayerPawn` 0))
    (if (== _roomtoupdate 0)
      (if (not (`self.BathroomHasBeenUpdated`))
        (set `self.BathroomHasBeenUpdated` true)
        (`/Game/Levels/Testlevel_TriggerZones_Jordan/BP_TriggerZones.Update Bathroom` _triggerzonesref 1)
        (`KismetSystemLibrary.PrintString` "The bathroom has been updated"))
      (elif (== _roomtoupdate 1)
        (if (not (`self.KitchenHasBeenUpdated`))
          (set `self.KitchenHasBeenUpdated` true)
          (`/Game/Levels/Testlevel_TriggerZones_Jordan/BP_TriggerZones.Update Kitchen` _triggerzonesref 1)
          (`KismetSystemLibrary.PrintString` "The kitchen has been updated"))
        (elif (== _roomtoupdate 2)
          (if (not (`self.LivingRoomHasBeenUpdated`))
            (set `self.LivingRoomHasBeenUpdated` true)
            (`/Game/Levels/Testlevel_TriggerZones_Jordan/BP_TriggerZones.Update LivingRoom` _triggerzonesref 1)
            (`KismetSystemLibrary.PrintString` "The living room has been updated"))
          (elif (== _roomtoupdate 3)
            (if (not (`self.OfficeHasBeenUpdated`))
              (set `self.OfficeHasBeenUpdated` true)
              (`/Game/Levels/Testlevel_TriggerZones_Jordan/BP_TriggerZones.Update Office` _triggerzonesref 1)
              (`KismetSystemLibrary.PrintString` "The office has been updated"))))))))

(fn `UserConstructionScript`)